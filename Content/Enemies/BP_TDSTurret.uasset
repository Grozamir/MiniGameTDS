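; BP_TDSTurret is an enemy turret whose Blueprint graph drives an in-world health bar.
; On BeginPlay it casts the Widget component's widget to BP_HealthProgressBarInWorld and caches its HealthPB progress bar.
; Every Tick it sets that bar's percent to the HealthComponent's current health divided by MaxHealth, polling rather than reacting to health-change events.
; The graph contains no targeting or firing logic, and the construction script is empty.
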(event EventTick
  (params (DeltaSeconds :type Float%20%28single-precision%29))
  (bind _self self)
  (bind _healthcomponent (Variables|Default|GetHealthComponent _self))
  (Progress|SetPercent (Variables|Default|GetHealth%20PB) (/ (Class|TDSHealthComponent|GetHealth _healthcomponent) (Variables|/Script/MiniGameTDS.TDSHealthComponent|GetMaxHealth _healthcomponent))))

(event EventBeginPlay
  (bind _asbp_health_progress_bar_in_world (Utilities|Casting|CastToBP_HealthProgressBarInWorld (UserInterface|GetWidget (Variables|Default|GetWidget))))
  (Variables|Default|SetHealth%20PB (Variables|/Game/UI/BP_HealthProgressBarInWorld.BP_HealthProgressBarInWorld_C|GetHealthPB _asbp_health_progress_bar_in_world)))

(fn ConstructionScript)